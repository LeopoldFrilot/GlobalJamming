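; BP_BeatMapController is a test-map Blueprint that records timestamped presses of number keys 1 to 4, apparently for authoring beat maps.
; Key presses append their digit to a per-frame string, so simultaneous presses share one entry.
; Tick appends non-empty frames with the current game time to a running total, prints it on screen, then clears the frame string.
; The recording is only printed, not saved.
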(event `self.ReceiveBeginPlay`
  (set `self.TotalString` ""))

(event `self.ReceiveTick`
  (params (DeltaSeconds :type "Float (single-precision)"))
  (`|ExecutionSequence`
    (:`then_0`
      (if (not (`KismetStringLibrary.IsEmpty` (`self.FrameString`)))
        (bind _output_get (set `self.TotalString` (`KismetStringLibrary.Concat_StrStr` (`self.TotalString`) (`KismetStringLibrary.Conv_DoubleToString` (`KismetSystemLibrary.GetGameTimeInSeconds`)) "+" (`self.FrameString`) ":")))
        (`KismetSystemLibrary.PrintString` _output_get true true (struct :`G` 0.66 :`B` 1.0 :`A` 1.0) 2.0 "werwer")))
    (:`then_1`
      (set `self.FrameString` ""))))

(event `Key|One`
  (params (Key :type "Key Structure"))
  (:`Pressed`
    (set `self.FrameString` (`KismetStringLibrary.Concat_StrStr` (`self.FrameString`) "1"))))

(event `Key|Two`
  (params (Key :type "Key Structure"))
  (:`Pressed`
    (set `self.FrameString` (`KismetStringLibrary.Concat_StrStr` (`self.FrameString`) "2"))))

(event `Key|Three`
  (params (Key :type "Key Structure"))
  (:`Pressed`
    (set `self.FrameString` (`KismetStringLibrary.Concat_StrStr` (`self.FrameString`) "3"))))

(event `Key|Four`
  (params (Key :type "Key Structure"))
  (:`Pressed`
    (set `self.FrameString` (`KismetStringLibrary.Concat_StrStr` (`self.FrameString`) "4"))))

(fn `UserConstructionScript`)