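; BP_Slime_Selector is a configurable slime actor from the Vefects Slime VFX pack that displays an animated skeletal slime in a chosen shape and look.
; The construction script resets actor scale, picks one of eight lit matcap materials from Variation, and picks a base, sphere, cube or torus mesh from Type.
; Each mesh gets its matching looping animation with random start position and play rate.
; On BeginPlay, RotateOnPlay optionally adds a random yaw.
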(event `self.ReceiveBeginPlay`
  (bind _skeletalmesh (`self.SkeletalMesh`))
  (bind (_returnvalue_roll _returnvalue_pitch _returnvalue_yaw) (`KismetMathLibrary.BreakRotator` (`SceneComponent.K2_GetComponentRotation` _skeletalmesh)))
  (if (`self.RotateOnPlay`)
    (`SceneComponent.K2_SetWorldRotation` _skeletalmesh (`KismetMathLibrary.MakeRotator` _returnvalue_roll _returnvalue_pitch (+ _returnvalue_yaw (`KismetMathLibrary.RandomFloatInRange` 0.0 360.0))) false false)))

(fn `UserConstructionScript`
  (bind _skeletalmesh (`self.SkeletalMesh`))
  (bind _skeletalmesh_2 (`self.SkeletalMesh`))
  (`self.SetActorScale3D` (1.0 1.0 1.0))
  (switch `int` (`self.Variation`)
    (:`Default`
      (`PrimitiveComponent.SetMaterial` _skeletalmesh 0 "/Game/Vefects/Slime_VFX/Slime/Materials/MI_VFX_Slime_Lit_Matcap_01.MI_VFX_Slime_Lit_Matcap_01" :!label _label))
    (:`0`
      (goto _label))
    (:`1`
      (`PrimitiveComponent.SetMaterial` _skeletalmesh 0 "/Game/Vefects/Slime_VFX/Slime/Materials/MI_VFX_Slime_Lit_Matcap_02.MI_VFX_Slime_Lit_Matcap_02"))
    (:`2`
      (`PrimitiveComponent.SetMaterial` _skeletalmesh 0 "/Game/Vefects/Slime_VFX/Slime/Materials/MI_VFX_Slime_Lit_Matcap_03.MI_VFX_Slime_Lit_Matcap_03"))
    (:`3`
      (`PrimitiveComponent.SetMaterial` _skeletalmesh 0 "/Game/Vefects/Slime_VFX/Slime/Materials/MI_VFX_Slime_Lit_Matcap_04.MI_VFX_Slime_Lit_Matcap_04"))
    (:`4`
      (`PrimitiveComponent.SetMaterial` _skeletalmesh 0 "/Game/Vefects/Slime_VFX/Slime/Materials/MI_VFX_Slime_Lit_Matcap_05.MI_VFX_Slime_Lit_Matcap_05"))
    (:`5`
      (`PrimitiveComponent.SetMaterial` _skeletalmesh 0 "/Game/Vefects/Slime_VFX/Slime/Materials/MI_VFX_Slime_Lit_Matcap_06.MI_VFX_Slime_Lit_Matcap_06"))
    (:`6`
      (`PrimitiveComponent.SetMaterial` _skeletalmesh 0 "/Game/Vefects/Slime_VFX/Slime/Materials/MI_VFX_Slime_Lit_Matcap_07.MI_VFX_Slime_Lit_Matcap_07"))
    (:`7`
      (`PrimitiveComponent.SetMaterial` _skeletalmesh 0 "/Game/Vefects/Slime_VFX/Slime/Materials/MI_VFX_Slime_Lit_Matcap_08.MI_VFX_Slime_Lit_Matcap_08")))
  (switch `int` (`self.Type`)
    (:`Default`
      (`SkinnedMeshComponent.SetSkinnedAssetAndUpdate` _skeletalmesh_2 "/Game/Vefects/Slime_VFX/Slime/Shared/Skeletal/SK_Slime_01_HD.SK_Slime_01_HD" false :!label _label_2)
      (set `SkeletalMeshComponent.AnimationData` (make `SingleAnimationPlayData` "/Game/Vefects/Slime_VFX/Slime/Shared/Skeletal/SK_Slime_01_HD_Anim.SK_Slime_01_HD_Anim" true true (`KismetMathLibrary.RandomFloatInRange` 0.0 1.0) (`KismetMathLibrary.RandomFloatInRange` 0.9 1.1)) _skeletalmesh_2))
    (:`0`
      (goto _label_2))
    (:`1`
      (`SkinnedMeshComponent.SetSkinnedAssetAndUpdate` _skeletalmesh_2 "/Game/Vefects/Slime_VFX/Slime/Shared/Skeletal/SK_Slime_Sphere_01_HD.SK_Slime_Sphere_01_HD" false)
      (set `SkeletalMeshComponent.AnimationData` (make `SingleAnimationPlayData` "/Game/Vefects/Slime_VFX/Slime/Shared/Skeletal/SK_Slime_Sphere_01_HD_Anim.SK_Slime_Sphere_01_HD_Anim" true true (`KismetMathLibrary.RandomFloatInRange` 0.0 1.0) (`KismetMathLibrary.RandomFloatInRange` 0.9 1.1)) _skeletalmesh_2))
    (:`2`
      (`SkinnedMeshComponent.SetSkinnedAssetAndUpdate` _skeletalmesh_2 "/Game/Vefects/Slime_VFX/Slime/Shared/Skeletal/SK_Slime_Cube_01_HD.SK_Slime_Cube_01_HD" false)
      (set `SkeletalMeshComponent.AnimationData` (make `SingleAnimationPlayData` "/Game/Vefects/Slime_VFX/Slime/Shared/Skeletal/SK_Slime_Cube_01_HD_Anim.SK_Slime_Cube_01_HD_Anim" true true (`KismetMathLibrary.RandomFloatInRange` 0.0 1.0) (`KismetMathLibrary.RandomFloatInRange` 0.9 1.1)) _skeletalmesh_2))
    (:`3`
      (`SkinnedMeshComponent.SetSkinnedAssetAndUpdate` _skeletalmesh_2 "/Game/Vefects/Slime_VFX/Slime/Shared/Skeletal/SK_Slime_Torus_01_HD.SK_Slime_Torus_01_HD" false)
      (set `SkeletalMeshComponent.AnimationData` (make `SingleAnimationPlayData` "/Game/Vefects/Slime_VFX/Slime/Shared/Skeletal/SK_Slime_Torus_01_HD_Anim.SK_Slime_Torus_01_HD_Anim" true true (`KismetMathLibrary.RandomFloatInRange` 0.0 1.0) (`KismetMathLibrary.RandomFloatInRange` 0.9 1.1)) _skeletalmesh_2))))