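; Slime VFX actor that spawns a Niagara slime effect over the surface of a configurable static mesh.
; The construction script picks the opaque or transparent Niagara system from the Transparent setting, then applies CustomMesh with the M_White material to the mesh component.
; That component is passed to Niagara as the User.StaticMesh override, with no active runtime event logic.
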(fn `UserConstructionScript`
  (bind _staticmesh (`self.StaticMesh`))
  (bind _niagara (`self.Niagara`))
  (switch `int` (`self.Transparent`)
    (:`Default`
      (`NiagaraComponent.SetAsset` _niagara "/Game/Vefects/Slime_VFX/Slime/Particles/NS_Slime_Surface_Spawn_Static_Mesh_01.NS_Slime_Surface_Spawn_Static_Mesh_01" true :!label _label))
    (:`0`
      (goto _label))
    (:`1`
      (`NiagaraComponent.SetAsset` _niagara "/Game/Vefects/Slime_VFX/Slime/Particles/NS_Slime_Surface_Spawn_Static_Mesh_01_Transparent.NS_Slime_Surface_Spawn_Static_Mesh_01_Transparent" true)))
  (`StaticMeshComponent.SetStaticMesh` _staticmesh (`self.CustomMesh`))
  (`PrimitiveComponent.SetMaterial` _staticmesh 0 "/Game/Vefects/Slime_VFX/Demo/Resources/Materials/M_White.M_White")
  (`NiagaraFunctionLibrary.OverrideSystemUserVariableStaticMeshComponent` (`self.Niagara`) "User.StaticMesh" (`self.StaticMesh`)))