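; Spline-based lane actor that spawns a BP_Bubble on a looping timer started at BeginPlay.
; The construction script tiles collision-free spline meshes along the spline, spacing them by the mesh's bounding-box X length and clamping tangents to that length.
; It also moves BPCMovementLocation to the spline's last point.
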(event `self.ReceiveBeginPlay`
  (`KismetSystemLibrary.K2_SetTimerDelegate` (delegate `LoopSPawn`) 2.0 true))

(event `LoopSPawn`
  (`self.SpawnBubble` "/Game/Blueprints/BP_Bubble.BP_Bubble_C"))

(fn `UserConstructionScript`
  (bind _spline (`self.Spline`))
  (bind _spline_2 (`self.Spline`))
  (bind (_returnvalue_min _returnvalue_max) (break `Box` (`StaticMesh.GetBoundingBox` (`self.SplineMesh`))))
  (bind _returnvalue_x (`KismetMathLibrary.BreakVector` (+ (`KismetMathLibrary.Vector_GetAbs` _returnvalue_min) (`KismetMathLibrary.Vector_GetAbs` _returnvalue_max))))
  (`|ExecutionSequence`
    (:`then_0`
      (bind _output_get (set `self.XLength` _returnvalue_x))
      (for _index (range (+ (`KismetMathLibrary.FTrunc` (/ (`SplineComponent.GetSplineLength` (`self.Spline`)) _output_get)) 1))
        (bind _returnvalue (`AddComponent|NODE_AddSplineMeshComponent-0`))
        (`PrimitiveComponent.SetCollisionEnabled` _returnvalue "NoCollision")
        (`SplineMeshComponent.SetForwardAxis` _returnvalue "X" true)
        (`StaticMeshComponent.SetStaticMesh` _returnvalue (`self.SplineMesh`))
        (bind _returnvalue_2 (* _index (`self.XLength`)))
        (bind _returnvalue_3 (* (+ _index 1) (`self.XLength`)))
        (`SplineMeshComponent.SetStartAndEnd` _returnvalue (`SplineComponent.GetLocationAtDistanceAlongSpline` _spline_2 _returnvalue_2 "Local") (`KismetMathLibrary.ClampVectorSize` (`SplineComponent.GetTangentAtDistanceAlongSpline` _spline_2 _returnvalue_2 "Local") 0.0 (`self.XLength`)) (`SplineComponent.GetLocationAtDistanceAlongSpline` _spline _returnvalue_3 "Local") (`KismetMathLibrary.ClampVectorSize` (`SplineComponent.GetTangentAtDistanceAlongSpline` _spline _returnvalue_3 "Local") 0.0 (`self.XLength`)) true)))
    (:`then_1`
      (`SceneComponent.K2_SetWorldLocation` (`self.BPC_MovementLocation`) (`SplineComponent.GetLocationAtSplinePoint` (`self.Spline`) (- (`SplineComponent.GetNumberOfSplinePoints` (`self.Spline`)) 1) "World") false false))))