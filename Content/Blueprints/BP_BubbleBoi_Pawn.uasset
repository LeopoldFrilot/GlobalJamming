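; BP_BubbleBoi_Pawn is the player input pawn that relays keyboard controls to the game.
; On BeginPlay it caches the first BP_GameWizard found in the level.
; Key releases tell the wizard to move left or right or switch directly to one of four lanes via letter or number keys.
; Space casts the wizard's BubbleBoi to BP_BubbleBoiCharacter and triggers ParryBubble.
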(event `self.ReceiveBeginPlay`
  (bind _outactors (`GameplayStatics.GetAllActorsOfClass` "/Game/Blueprints/BP_GameWizard.BP_GameWizard_C"))
  (set `self.GameWizard` (`|GetArrayItem` _outactors)))

(event `Key|Right`
  (params (Key :type "Key Structure"))
  (:`Released`
    (`/Game/Blueprints/BP_GameWizard.MoveRight` (`self.GameWizard`))))

(event `Key|Left`
  (params (Key :type "Key Structure"))
  (:`Released`
    (`/Game/Blueprints/BP_GameWizard.MoveLeft` (`self.GameWizard`))))

(event `Key|A`
  (params (Key :type "Key Structure"))
  (:`Released`
    (`/Game/Blueprints/BP_GameWizard.SwitchToLane` (`self.GameWizard`) 0 :!label _label)))

(event `Key|One`
  (params (Key :type "Key Structure"))
  (:`Released`
    (goto _label)))

(event `Key|S`
  (params (Key :type "Key Structure"))
  (:`Released`
    (`/Game/Blueprints/BP_GameWizard.SwitchToLane` (`self.GameWizard`) 1 :!label _label_2)))

(event `Key|Two`
  (params (Key :type "Key Structure"))
  (:`Released`
    (goto _label_2)))

(event `Key|D`
  (params (Key :type "Key Structure"))
  (:`Released`
    (`/Game/Blueprints/BP_GameWizard.SwitchToLane` (`self.GameWizard`) 2 :!label _label_3)))

(event `Key|Three`
  (params (Key :type "Key Structure"))
  (:`Released`
    (goto _label_3)))

(event `Key|F`
  (params (Key :type "Key Structure"))
  (:`Released`
    (`/Game/Blueprints/BP_GameWizard.SwitchToLane` (`self.GameWizard`) 3 :!label _label_4)))

(event `Key|Four`
  (params (Key :type "Key Structure"))
  (:`Released`
    (goto _label_4)))

(event `Key|SpaceBar`
  (params (Key :type "Key Structure"))
  (:`Released`
    (bind _asbp_bubble_boi_character (cast `/Game/Blueprints/BP_BubbleBoiCharacter` (`/Game/Blueprints/BP_GameWizard.BubbleBoi` (`self.GameWizard`))))
    (`/Game/Blueprints/BP_BubbleBoiCharacter.ParryBubble` _asbp_bubble_boi_character)))

(fn `UserConstructionScript`)