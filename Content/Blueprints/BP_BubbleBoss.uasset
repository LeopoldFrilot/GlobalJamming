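; Boss actor that takes damage when bubbles hit it.
; On overlap with a BP_Bubble_Base, it forwards the bubble's damage to BP_GameplayGameMode, plays a sound and pops the bubble.
; Damage handling is delegated to the game mode through DealDamageToBoss.
; BeginPlay caches the first BP_GameWizard in the level, though the graph never uses that reference afterward.
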(event `self.ReceiveBeginPlay`
  (bind _outactors (`GameplayStatics.GetAllActorsOfClass` "/Game/Blueprints/BP_GameWizard.BP_GameWizard_C"))
  (set `self.GameWizard` (`|GetArrayItem` _outactors)))

(event `self.ReceiveActorBeginOverlap`
  (params (OtherActor :type "Actor Object Reference"))
  (bind _asbp_bubble_base (cast `/Game/Blueprints/Bubbles/BP_Bubble_Base` OtherActor))
  (bind _asbp_gameplay_game_mode (cast `/Game/Blueprints/BP_GameplayGameMode` (`GameplayStatics.GetGameMode`)))
  (`BBGameMode.DealDamageToBoss` _asbp_gameplay_game_mode (`/Game/Blueprints/Bubbles/BP_Bubble_Base.Damage` _asbp_bubble_base))
  (`GameplayStatics.PlaySound2D` null 1.0 1.0 0.0 null null)
  (`Bubble.PopBubble` _asbp_bubble_base))

(fn `UserConstructionScript`)