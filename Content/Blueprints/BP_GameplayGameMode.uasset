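; Gameplay game mode that starts the game and reports player and boss combat events as on-screen debug text.
; BeginPlay binds handlers to the player and boss hurt and died dispatchers, then calls StartGame, which runs the parent version and broadcasts OnGameStart.
; The handlers only print messages, with keyed prints for remaining health; deaths trigger no further game logic here.
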(event `self.ReceiveBeginPlay`
  (add `self.OnPlayerDied` (delegate `PlayerDied`))
  (add `self.OnPlayerHurt` (delegate `OnPlayerHurt_Event`))
  (add `self.OnBossHurt` (delegate `OnBossHurt_Event`))
  (add `self.OnBossDied` (delegate `OnBossDied_Event`))
  (`self.StartGame`))

(event `OnBossHurt_Event` :!signature `self.OnBossHurt`
  (params (Previous :type Integer) (New :type Integer))
  (`KismetSystemLibrary.PrintString` (`KismetStringLibrary.Concat_StrStr` "Boss got hurt! \nHealth left: " (`KismetStringLibrary.Conv_IntToString` New)) true true (struct :`G` 0.805828 :`B` 1.0 :`A` 1.0) 10.0 "BossHealth"))

(event `OnBossDied_Event`
  (`KismetSystemLibrary.PrintString` "Boss DIED" true true (struct :`G` 1.0 :`B` 0.122982 :`A` 1.0) 100.0))

(event `PlayerDied`
  (`KismetSystemLibrary.PrintString` "PLAYER DIED" true true (struct :`R` 1.0 :`A` 1.0) 100.0))

(event `OnPlayerHurt_Event` :!signature `self.OnPlayerHurt`
  (params (Previous :type Integer) (New :type Integer))
  (`KismetSystemLibrary.PrintString` (`KismetStringLibrary.Concat_StrStr` "You got hurt! \nHealth left: " (`KismetStringLibrary.Conv_IntToString` New)) true true (struct :`R` 1.0 :`G` 0.687129 :`A` 1.0) 10.0 "Health"))

(event `self.StartGame`
  (`parent.StartGame`)
  (`self.OnGameStart`))

(fn `UserConstructionScript`)