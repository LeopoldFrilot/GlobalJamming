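; BP_GameWizard runs a lane-based bubble game, starting music and spawning when the game mode signals start.
; Each tick it spawns LevelLines rows into Lanes on a one-second countdown, falling back to armored bubbles when rows run out.
; It teleports BubbleBoi between active lanes and lerps parried bubbles toward BubbleBoss.
; ExtractBeatmap parses strings into timestamped rows, but is uncalled here, and spawning ignores timestamps.
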(event `self.ReceiveBeginPlay`
  (bind _asbp_gameplay_game_mode (cast `/Game/Blueprints/BP_GameplayGameMode` (`GameplayStatics.GetGameMode`)))
  (add `/Game/Blueprints/BP_GameplayGameMode.OnGameStart` _asbp_gameplay_game_mode (delegate `OnGameStart_Event`))
  (`KismetArrayLibrary.Array_Clear` (`self.LevelLines`)))

(event `OnGameStart_Event`
  (`self.RefreshLanes`)
  (`self.SwitchToLane` 1)
  (set `self.Started` true)
  (bind _returnvalue (`GameplayStatics.SpawnSound2D` "/Game/Audio/Jam1.Jam1" 1.0 1.0 0.0 null))
  (set `self.Jam` _returnvalue))

(event `self.ReceiveTick`
  (params (DeltaSeconds :type "Float (single-precision)"))
  (if (`self.Started`)
    (`self.ProgressLevel`)
    (`self.MoveBubbles`)))

(event `self.ReceiveEndPlay`
  (params (EndPlayReason :type "EEndPlayReason Enum" :default "Destroyed"))
  (bind _jam (`self.Jam`))
  (`/Engine/EditorBlueprintResources/StandardMacros.IsValid` _jam
    (:`Is Valid`
      (`AudioComponent.Stop` _jam)
      (`ActorComponent.K2_DestroyComponent` _jam))))

(event `RefreshLanes`
  (for (_array_element _array_index) (`self.Lanes`)
    (`/Engine/EditorBlueprintResources/StandardMacros.IsValid` _array_element
      (:`Is Valid`
        (switch `int` (`self.Level`)
          (:`0`
            (bind _output_get (set `/Game/Blueprints/BP_BubbleLane.Active` (< _array_index 3) _array_element))
            (`self.SetActorHiddenInGame` _array_element (not _output_get))))))))

(event `SwitchToLane`
  (params (NewLane :type Integer))
  (bind _bubbleboi (`self.BubbleBoi`))
  (bind (_returnvalue_x _returnvalue_y _returnvalue_z) (`KismetMathLibrary.BreakVector` (`self.K2_GetActorLocation` _bubbleboi)))
  (bind _output (`|GetArrayItem` (`self.Lanes`) NewLane))
  (bind (_returnvalue_x_2 _returnvalue_y_2) (`KismetMathLibrary.BreakVector` (`SceneComponent.K2_GetComponentLocation` (`/Game/Blueprints/BP_BubbleLane.BPC_MovementLocation` _output))))
  (if (and (not (`/Game/Blueprints/BP_BubbleBoiCharacter.IsInParry` (cast `/Game/Blueprints/BP_BubbleBoiCharacter` (`self.BubbleBoi`) :!pure true))) (`KismetArrayLibrary.Array_IsValidIndex` (`self.Lanes`) NewLane))
    (`/Engine/EditorBlueprintResources/StandardMacros.IsValid` _output
      (:`Is Valid`
        (if (`/Game/Blueprints/BP_BubbleLane.Active` _output)
          (`self.K2_SetActorLocation` _bubbleboi (`KismetMathLibrary.MakeVector` _returnvalue_x_2 _returnvalue_y_2 _returnvalue_z) false true)
          (set `self.CurrentLane` NewLane)
          (`GameplayStatics.PlaySound2D` "/Game/Audio/Liquid_Water_Water_Drop_02_.Liquid_Water_Water_Drop_02_" 1.0 1.0 0.0 null null))))))

(event `MoveRight`
  (`self.SwitchToLane` (+ (`self.CurrentLane`) 1)))

(event `MoveLeft`
  (`self.SwitchToLane` (- (`self.CurrentLane`) 1)))

(event `ParryBubble`
  (params (Bubble :type "/Game/Blueprints/Bubbles/BP_Bubble_Base Object Reference"))
  (set `/Game/Blueprints/Bubbles/BP_Bubble_Base.Parried` true Bubble)
  (for _array_element (`self.Lanes`)
    (`/Engine/EditorBlueprintResources/StandardMacros.IsValid` _array_element
      (:`Is Valid`
        (`BBBubbleLane.RemoveBubble` _array_element Bubble))))
  (`self.Launch at Boss` Bubble))

(event `Launch at Boss`
  (params (`Bubble Target` :type "/Game/Blueprints/Bubbles/BP_Bubble_Base Object Reference"))
  (`KismetArrayLibrary.Array_Add` (`self.LaunchedBubbles`) `Bubble Target`))

(fn `ExtractBeatmap`
  (locals (NewLocalVar :type String) (Bubbles :type "Array of /Game/Blueprints/Bubbles/BP_Bubble_Base Class Reference") (Timestamp :type String) (Beats :type String))
  (bind _beats (`local.Beats`))
  (bind (_lefts _rights _returnvalue) (`KismetStringLibrary.Split` (`self.LevelLineBeatmap`) ":"))
  (set `local.NewLocalVar` (`self.LevelLineBeatmap`))
  (while (`KismetStringLibrary.IsEmpty` (`local.NewLocalVar`))
    (if _returnvalue
      (`KismetArrayLibrary.Array_Add` (`self.Lines`) _lefts)
      (set `local.NewLocalVar` _rights)))
  (`KismetArrayLibrary.Array_Clear` (`local.Bubbles`))
  (for _array_element (`self.Lines`)
    (bind (_lefts_2 _rights_2) (`KismetStringLibrary.Split` _array_element "+"))
    (set `local.Timestamp` _lefts_2)
    (set `local.Beats` _rights_2)
    (set `local.Bubbles` (`|MakeArray` null null null null :!type "/Game/Blueprints/Bubbles/BP_Bubble_Base Class Reference"))
    (`|ExecutionSequence`
      (:`then_0`
        (if (`KismetStringLibrary.Contains` _beats "1")
          (`KismetArrayLibrary.Array_Set` (`local.Bubbles`) 0 "/Game/Blueprints/Bubbles/BP_NormalBubble.BP_NormalBubble_C")))
      (:`then_1`
        (if (`KismetStringLibrary.Contains` _beats "2")
          (`KismetArrayLibrary.Array_Set` (`local.Bubbles`) 1 "/Game/Blueprints/Bubbles/BP_NormalBubble.BP_NormalBubble_C")))
      (:`then_2`
        (if (`KismetStringLibrary.Contains` _beats "3")
          (`KismetArrayLibrary.Array_Set` (`local.Bubbles`) 2 "/Game/Blueprints/Bubbles/BP_NormalBubble.BP_NormalBubble_C")))
      (:`then_3`
        (if (`KismetStringLibrary.Contains` _beats "4")
          (`KismetArrayLibrary.Array_Set` (`local.Bubbles`) 3 "/Game/Blueprints/Bubbles/BP_NormalBubble.BP_NormalBubble_C")))
      (:`then_4`
        (`KismetArrayLibrary.Array_Add` (`self.LevelLines`) (make `/Game/Blueprints/F_LevelLine` (`KismetStringLibrary.Conv_StringToDouble` (`local.Timestamp`)) (`local.Bubbles`)))))))

(fn `MoveBubbles`
  (bind _launchedbubbles (`self.LaunchedBubbles`))
  (for (_array_element _array_index) _launchedbubbles
    (`/Engine/EditorBlueprintResources/StandardMacros.IsValid` _array_element
      (:`Is Valid`
        (`self.K2_SetActorLocation` _array_element (`KismetMathLibrary.VLerp` (`self.K2_GetActorLocation` _array_element) (`self.K2_GetActorLocation` (`self.BubbleBoss`)) (* (`GameplayStatics.GetWorldDeltaSeconds`) (`self.LaunchSpeed`))) false false))
      (:`Is Not Valid`
        (`KismetArrayLibrary.Array_Remove` _launchedbubbles _array_index)))))

(fn `ProgressLevel`
  (bind _levelindex (`self.LevelIndex`))
  (bind (_output_timestamp _output_bubbles) (break `/Game/Blueprints/F_LevelLine` (`|GetArrayItem` (`self.LevelLines`) _levelindex)))
  (if (<= (`self.TimeTillSpawn`) 0.0)
    (if (`KismetArrayLibrary.Array_IsValidIndex` (`self.LevelLines`) _levelindex)
      (for (_array_element _array_index) _output_bubbles
        (if (`KismetSystemLibrary.IsValidClass` _array_element)
          (`BBBubbleLane.SpawnBubble` (`|GetArrayItem` (`self.Lanes`) _array_index) _array_element)))
      (`/Engine/EditorBlueprintResources/StandardMacros.IncrementInt` (`self.LevelIndex`)
        (:`  `
          (switch `int` (`self.Level`)
            (:`Default`
              _)
            (:`0`
              _))
          (set `self.TimeTillSpawn` 1.0)))
      (else
        (for _array_element_2 (`self.Lanes`)
          (`BBBubbleLane.SpawnBubble` _array_element_2 "/Game/Blueprints/Bubbles/BP_ArmoredBubble.BP_ArmoredBubble_C"))
        (set `self.TimeTillSpawn` 1.0)))
    (else
      (set `self.TimeTillSpawn` (- (`self.TimeTillSpawn`) (`GameplayStatics.GetWorldDeltaSeconds`))))))

(fn `UserConstructionScript`)